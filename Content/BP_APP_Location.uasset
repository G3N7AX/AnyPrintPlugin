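; BP_APP_Location is an actor that shuttles endlessly between two referenced actors, PointOne and PointTwo, starting on BeginPlay.
; Two timelines alternate, each starting the other when finished, with the actor's location printed at every handover.
; Each update lerps from the current location rather than a cached start, so the timeline alpha compounds instead of mapping directly to position along the path.
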(event `self.ReceiveBeginPlay`
  (`parent.ReceiveBeginPlay`)
  (`self.MoveForward`))

(event `MoveForward`
  (bind (_direction _alpha) (`Timeline|TL_MoveObjectForwards` :!via `PlayFromStart`)
    (:`Update`
      (`self.K2_SetActorLocation` (`KismetMathLibrary.VLerp` (`self.K2_GetActorLocation`) (`self.K2_GetActorLocation` (`self.PointOne`)) _alpha)))
    (:`Finished`
      (`self.PrintLocation`)
      (`self.MoveBackwards`))))

(event `MoveBackwards`
  (bind (_direction _alpha) (`Timeline|TL_MoveObjectBackwards` :!via `PlayFromStart`)
    (:`Update`
      (`self.K2_SetActorLocation` (`KismetMathLibrary.VLerp` (`self.K2_GetActorLocation`) (`self.K2_GetActorLocation` (`self.PointTwo`)) _alpha)))
    (:`Finished`
      (`self.PrintLocation`)
      (`self.MoveForward`))))

(event `PrintLocation`
  (`DebugFunctionLibrary.PrintAnything` (`KismetStringLibrary.Conv_VectorToString` (`self.K2_GetActorLocation`))))

(fn `UserConstructionScript`
  (`parent.UserConstructionScript`))